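; Weapon pickup actor that grants its Item and Quantity to a ThirdPersonCharacter that overlaps its Hitbox.
; On overlap it shows a WeaponObtainedHUD widget, then looks up the item's WeaponTable row by enum name.
; Switchable weapons add Quantity to the character's enum-indexed ItemsGathered array, while others overwrite BestMelee without comparison.
; The actor destroys itself only when the row is found.
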(event OnComponentBeginOverlap(Hitbox)
  (params (OverlappedComponent :type Primitive%20Component%20Object%20Reference) (OtherActor :type Actor%20Object%20Reference) (OtherComp :type Primitive%20Component%20Object%20Reference) (OtherBodyIndex :type Integer) (bFromSweep :type Boolean) (SweepResult :type Hit%20Result%20Structure%20%28by%20ref%29))
  (bind _item (Variables|Default|GetItem))
  (bind _returnvalue (Math|Conversions|ToInteger(Byte) _item))
  (bind _asthird_person_character (Utilities|Casting|CastToThirdPersonCharacter OtherActor))
  ;[1 0 0.08212] Create Widget
  (bind _returnvalue_2 (UserInterface|CreateWidget "/Game/3DBP/Blueprints/WeaponObtainedHUD.WeaponObtainedHUD_C" 0 (Variables|Default|GetQuantity) (Variables|Default|GetItem)))
  (UserInterface|Viewport|AddtoViewport _returnvalue_2 0)
  (bind _returnvalue_3 (Utilities|GetDataTableRow "/Game/2DSideScrollerBP/Blueprints/WeaponSystem/WeaponTable.WeaponTable" (Utilities|String|StringToName (Utilities|String|EnumtoString (Variables|Default|GetItem))))
    (:then
      (if (.Switchable (Utilities|Struct|BreakWeaponInfo _returnvalue_3))
        ;[1 1 1] Wrote at 2am, I have no idea
        (if (Utilities|Array|IsValidIndex (Variables|/Game/3DBP/Blueprints/ThirdPersonCharacter.ThirdPersonCharacter_C|GetItems%20Gathered _asthird_person_character) _returnvalue)
          (Variables|Default|SetQuantity (+ (Variables|Default|GetQuantity) (Utilities|Array|Get(acopy) (Variables|/Game/3DBP/Blueprints/ThirdPersonCharacter.ThirdPersonCharacter_C|GetItems%20Gathered _asthird_person_character) _returnvalue))))
        (Utilities|Array|SetArrayElem (Variables|/Game/3DBP/Blueprints/ThirdPersonCharacter.ThirdPersonCharacter_C|GetItems%20Gathered _asthird_person_character) _returnvalue (Variables|Default|GetQuantity) true)
        (else
          ;[1 1 1] We only have 2 weapons currently so it is obvious that it will be strictly better
          (Variables|/Game/3DBP/Blueprints/ThirdPersonCharacter.ThirdPersonCharacter_C|SetBestMelee _asthird_person_character (Variables|Default|GetItem))))
      (Actor|DestroyActor))))

(event EventBeginPlay)

(event Collision|EventActorBeginOverlap
  (params (OtherActor :type Actor%20Object%20Reference)))

(event EventTick
  (params (DeltaSeconds :type Float%20%28single-precision%29)))

(fn ConstructionScript)