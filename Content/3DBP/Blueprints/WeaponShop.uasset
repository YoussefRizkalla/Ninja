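; Weapon shop actor that tells the player character when it is within range of the shop.
; Hitbox overlap with a ThirdPersonCharacter shows InfoText, sets the character's InRangeOfShop flag and registers this shop as its NearestShop.
; Leaving the hitbox hides the text and clears the flag but leaves NearestShop set.
; The shop itself contains no purchase logic.
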(event OnComponentBeginOverlap(Hitbox)
  (params (OverlappedComponent :type Primitive%20Component%20Object%20Reference) (OtherActor :type Actor%20Object%20Reference) (OtherComp :type Primitive%20Component%20Object%20Reference) (OtherBodyIndex :type Integer) (bFromSweep :type Boolean) (SweepResult :type Hit%20Result%20Structure%20%28by%20ref%29))
  (bind _asthird_person_character (Utilities|Casting|CastToThirdPersonCharacter OtherActor))
  (Rendering|SetVisibility (Variables|Default|GetInfo%20Text) true false)
  (Variables|/Game/3DBP/Blueprints/ThirdPersonCharacter.ThirdPersonCharacter_C|SetInRangeOfShop _asthird_person_character true)
  (Variables|/Game/3DBP/Blueprints/ThirdPersonCharacter.ThirdPersonCharacter_C|SetNearestShop _asthird_person_character self))

(event OnComponentEndOverlap(Hitbox)
  (params (OverlappedComponent :type Primitive%20Component%20Object%20Reference) (OtherActor :type Actor%20Object%20Reference) (OtherComp :type Primitive%20Component%20Object%20Reference) (OtherBodyIndex :type Integer))
  (bind _asthird_person_character (Utilities|Casting|CastToThirdPersonCharacter OtherActor))
  (Rendering|SetVisibility (Variables|Default|GetInfo%20Text) false false)
  (Variables|/Game/3DBP/Blueprints/ThirdPersonCharacter.ThirdPersonCharacter_C|SetInRangeOfShop _asthird_person_character false))

(event EventBeginPlay)

(event Collision|EventActorBeginOverlap
  (params (OtherActor :type Actor%20Object%20Reference)))

(event EventTick
  (params (DeltaSeconds :type Float%20%28single-precision%29)))

(fn ConstructionScript)